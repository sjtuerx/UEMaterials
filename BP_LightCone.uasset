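; BP_LightCone is a projector-style light cone actor built entirely in its Construction Script.
; A SceneCaptureComponent2D, hiding the actor itself, captures into a newly created render target.
; The cone mesh gets a dynamic LightConeMaterial, is scaled by Size and Length, and is offset along its local Z axis.
; UpdateMaterialValues passes the actor's location and axes, capture FOV and render target to that material as projector parameters.
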(fn `UpdateMaterialValues`
  (bind _mid (`self.MID`))
  (bind _scenecapturecomponent2d (`self.SceneCaptureComponent2D`))
  (`MaterialInstanceDynamic.SetVectorParameterValue` _mid "ProjectorLocation" (`KismetMathLibrary.Conv_VectorToLinearColor` (`self.K2_GetActorLocation`)))
  (`MaterialInstanceDynamic.SetVectorParameterValue` _mid "ProjectorForward" (`KismetMathLibrary.Conv_VectorToLinearColor` (`self.GetActorForwardVector`)))
  (`MaterialInstanceDynamic.SetVectorParameterValue` _mid "ProjectorRight" (`KismetMathLibrary.Conv_VectorToLinearColor` (`self.GetActorRightVector`)))
  (`MaterialInstanceDynamic.SetVectorParameterValue` _mid "ProjectorUp" (`KismetMathLibrary.Conv_VectorToLinearColor` (`self.GetActorUpVector`)))
  (`MaterialInstanceDynamic.SetScalarParameterValue` _mid "ProjectorFOV" (`SceneCaptureComponent2D.FOVAngle` _scenecapturecomponent2d))
  (`MaterialInstanceDynamic.SetTextureParameterValue` _mid "ProjectorTexture" (`SceneCaptureComponent2D.TextureTarget` _scenecapturecomponent2d)))

(fn `UserConstructionScript`
  (bind _scenecapturecomponent2d (`self.SceneCaptureComponent2D`))
  (bind _length (`self.Length`))
  (bind _staticmesh (`self.StaticMesh`))
  (bind _size (`self.Size`))
  (`|ExecutionSequence`
    (:`then_0`
      (`KismetArrayLibrary.Array_Add` (`SceneCaptureComponent.HiddenActors` _scenecapturecomponent2d) self))
    (:`then_1`
      (bind _returnvalue (`KismetRenderingLibrary.CreateRenderTarget2D` 256))
      (set `SceneCaptureComponent2D.TextureTarget` _returnvalue _scenecapturecomponent2d))
    (:`then_2`
      (bind _returnvalue_2 (`KismetMaterialLibrary.CreateDynamicMaterialInstance` (`self.LightConeMaterial`)))
      (bind _output_get (set `self.MID` _returnvalue_2))
      (`PrimitiveComponent.SetMaterial` (`self.StaticMesh`) 0 _output_get))
    (:`then_3`
      (`SceneComponent.SetWorldScale3D` _staticmesh (`KismetMathLibrary.MakeVector` _size _size _length))
      (`SceneComponent.K2_AddLocalOffset` _staticmesh (`KismetMathLibrary.MakeVector` 0.0 0.0 (+ (* (/ _length 2.0) -100.0) 20.0)) false false))
    (:`then_4`
      (`self.UpdateMaterialValues`))))